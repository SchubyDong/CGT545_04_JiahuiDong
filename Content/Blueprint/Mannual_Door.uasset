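; Manual door actor that swings its Door component 90 degrees open or closed on the Flip_Door input action.
; A FlipFlop alternates playing and reversing a timeline that drives the rotation lerp.
; Door_Collision overlap calls EnableInput and DisableInput on the entering or leaving BP_FirstPersonCharacter itself, with no call on the door.
; The Open_Door and Close_Door functions are empty stubs.
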(event OnComponentBeginOverlap(Door_Collision)
  (params (OverlappedComponent :type Primitive%20Component%20Object%20Reference) (OtherActor :type Actor%20Object%20Reference) (OtherComp :type Primitive%20Component%20Object%20Reference) (OtherBodyIndex :type Integer) (bFromSweep :type Boolean) (SweepResult :type Hit%20Result%20Structure%20%28by%20ref%29))
  (bind _asbp_first_person_character (Utilities|Casting|CastToBP_FirstPersonCharacter OtherActor))
  (Input|EnableInput _asbp_first_person_character 0))

(event OnComponentEndOverlap(Door_Collision)
  (params (OverlappedComponent :type Primitive%20Component%20Object%20Reference) (OtherActor :type Actor%20Object%20Reference) (OtherComp :type Primitive%20Component%20Object%20Reference) (OtherBodyIndex :type Integer))
  (bind _asbp_first_person_character (Utilities|Casting|CastToBP_FirstPersonCharacter OtherActor))
  (Input|DisableInput _asbp_first_person_character 0))

(event EventBeginPlay)

(event Collision|EventActorBeginOverlap
  (params (OtherActor :type Actor%20Object%20Reference)))

(event EventTick
  (params (DeltaSeconds :type Float%20%28single-precision%29)))

(event Input|ActionEvents|InputActionFlip_Door
  (params (Key :type Key%20Structure :default "None"))
  (:Pressed
    (Utilities|FlowControl|FlipFlop
      (:A
        (bind _newtrack_0 (Timeline|Timeline_0 Play)
          (:Update
            (Transformation|SetRelativeRotation (Variables|Default|GetDoor) (Math|Rotator|Lerp(Rotator) "0, 0, 0" "0,90.000000, 0" _newtrack_0) false false))))
      (:B
        (Timeline|Timeline_0 Reverse)))))

(fn ConstructionScript)

(fn OpenDoor)

(fn CloseDoor)